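; BP_Turret is an enemy turret actor that shows its health widget while a BP_Drone is inside its detection zone.
; On BeginPlay it passes itself to the WB_TurretHealth instance in its widget component.
; DetectionZone begin and end overlaps with a BP_Drone toggle that widget component's visibility.
; The graph contains no targeting, firing or damage logic.
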(event `self.ReceiveBeginPlay`
  (bind _aswb_turret_health (cast `/Game/Widget/WB_TurretHealth` (`WidgetComponent.GetUserWidgetObject` (`self.Widget`))))
  (set `/Game/Widget/WB_TurretHealth.Turret` self _aswb_turret_health))

(event `self.DetectionZone.OnComponentBeginOverlap`
  (params (OverlappedComponent :type "PrimitiveComponent Object Reference") (OtherActor :type "Actor Object Reference") (OtherComp :type "PrimitiveComponent Object Reference") (OtherBodyIndex :type Integer) (bFromSweep :type Boolean) (SweepResult :type "HitResult Structure (by ref)"))
  (cast `/Game/Blueprints/Character/BP_Drone` OtherActor)
  (`SceneComponent.SetVisibility` (`self.Widget`) true false))

(event `self.DetectionZone.OnComponentEndOverlap`
  (params (OverlappedComponent :type "PrimitiveComponent Object Reference") (OtherActor :type "Actor Object Reference") (OtherComp :type "PrimitiveComponent Object Reference") (OtherBodyIndex :type Integer))
  (cast `/Game/Blueprints/Character/BP_Drone` OtherActor)
  (`SceneComponent.SetVisibility` (`self.Widget`) false false))

(fn `UserConstructionScript`)